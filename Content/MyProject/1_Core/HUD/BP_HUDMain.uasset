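; BP_HUDMain is a HUD Blueprint that adds the WB_HUD widget to the viewport and provides drag-box selection of BP_Character units.
; StartSelection and DrawHUD capture the drag corners from viewport mouse position times viewport scale to correct for scaling.
; Past a minimum drag length, DrawHUD draws a translucent rectangle and gathers characters inside it.
; StopSelection then replaces the BP_Controler unit selection with those characters.
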(event `self.ReceiveBeginPlay`
  (bind _asbp_controler (cast `/Game/MyProject/1_Core/Character/BP_Controler` (`GameplayStatics.GetPlayerController` 0)))
  (set `self.As BP Controler` _asbp_controler)
  (bind _returnvalue (`|CreateWidget` "/Game/MyProject/6_UI/WB_HUD.WB_HUD_C"))
  (`UserWidget.AddToViewport` _returnvalue 0))

(event `/Game/MyProject/1_Core/HUD/BPI_SelectionUnit.StartSelection`
  ;[1 1 1] select unit
  ;;[1 1 1] solve problem with scale
  (bind _returnvalue (`WidgetLayoutLibrary.GetMousePositionOnViewport`))
  (bind (_returnvalue_x _returnvalue_y) (`KismetMathLibrary.BreakVector2D` (* _returnvalue (`WidgetLayoutLibrary.GetViewportScale`))))
  (set `self.BeginnigPoint` (`KismetMathLibrary.MakeVector2D` _returnvalue_x _returnvalue_y))
  (set `self.bDrawing` true))

(event `/Game/MyProject/1_Core/HUD/BPI_SelectionUnit.StopSelection`
  ;[1 1 1] select unit
  (set `self.bDrawing` false)
  (if (`self.bMarquee`)
    (`/Game/MyProject/1_Core/Character/BP_Controler.ClearUnitSelection` (`self.As BP Controler`))
    (for _array_element (`self.ActorSelected`)
      (bind _asbp_character (cast `/Game/MyProject/1_Core/Character/BP_Character` _array_element))
      (`/Game/MyProject/1_Core/Character/BP_Controler.AddUnitSelection` (`self.As BP Controler`) _asbp_character))
    (set `self.bMarquee` false)))

(event `self.ReceiveDrawHUD`
  (params (SizeX :type Integer) (SizeY :type Integer))
  (bind (_beginnigpoint_x _beginnigpoint_y) (`KismetMathLibrary.BreakVector2D` (`self.BeginnigPoint`)))
  (bind (_endpoint_x _endpoint_y) (`KismetMathLibrary.BreakVector2D` (`self.EndPoint`)))
  ;[1 1 1] select unit
  (if (`self.bDrawing`)
    ;;[1 1 1] solve problem with scale
    (bind _returnvalue (`WidgetLayoutLibrary.GetMousePositionOnViewport`))
    (bind (_returnvalue_x _returnvalue_y) (`KismetMathLibrary.BreakVector2D` (* _returnvalue (`WidgetLayoutLibrary.GetViewportScale`))))
    (set `self.EndPoint` (`KismetMathLibrary.MakeVector2D` _returnvalue_x _returnvalue_y))
    (if (> (`KismetMathLibrary.VSize2D` (- (`self.BeginnigPoint`) (`self.EndPoint`))) (`self.VektorLenght`))
      (`self.DrawRect` (struct :`R` 0.45026 :`G` 0.95 :`B` 0.551745 :`A` 0.5) _beginnigpoint_x _beginnigpoint_y (- _endpoint_x _beginnigpoint_x) (- _endpoint_y _beginnigpoint_y))
      (set `self.bMarquee` true)
      (set `self.ActorSelected` (`self.GetActorsInSelectionRectangle` "/Game/MyProject/1_Core/Character/BP_Character.BP_Character_C" (`self.BeginnigPoint`) (`self.EndPoint`))))))

(fn `UserConstructionScript`)