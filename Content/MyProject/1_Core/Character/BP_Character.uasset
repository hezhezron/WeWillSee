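; Clickable character for mouse-driven unit selection and orders, with a Niagara targeting marker that also shows by default on non-player characters.
; Left-click toggles a player character in BP_Controler's selection, using marker visibility as the selected state.
; Right-click makes selected units target this character, writing a nearby navigable point and action to their AI blackboards.
; Health component death triggers a one-time ragdoll; Attack and damage handlers are empty.
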(event `UnitSelected`
  (params (bUnitSelected :type Boolean))
  (`SceneComponent.SetVisibility` (`self.NS_Targeting_Player_Select`) bUnitSelected true))

(event `self.ReceiveActorOnClicked`
  (params (ButtonPressed :type "Key Structure"))
  (if (and (== ButtonPressed "LeftMouseButton") (`self.bPlayerCharacter`))
    (bind _asbp_controler (cast `/Game/MyProject/1_Core/Character/BP_Controler` (`GameplayStatics.GetPlayerController` 0)))
    (set `self.As BP Controler` _asbp_controler)
    (if (`SceneComponent.IsVisible` (`self.NS_Targeting_Player_Select`))
      (`/Game/MyProject/1_Core/Character/BP_Controler.DeleteUnitSelection` (`self.As BP Controler`) self)
      (else
        (`/Game/MyProject/1_Core/Character/BP_Controler.AddUnitSelection` (`self.As BP Controler`) self)))
    (elif (== ButtonPressed "RightMouseButton")
      (bind _asbp_controler_2 (cast `/Game/MyProject/1_Core/Character/BP_Controler` (`GameplayStatics.GetPlayerController` 0)))
      (for _array_element (`/Game/MyProject/1_Core/Character/BP_Controler.SelectedUnit` _asbp_controler_2)
        (set `/Game/MyProject/1_Core/Character/BP_Character.TargetActor` self _array_element)
        (bind _blackboard (`AIController.Blackboard` (`AIBlueprintHelperLibrary.GetAIController` _array_element)))
        (`BlackboardComponent.SetValueAsVector` _blackboard "TravelLocation" (`NavigationSystemV1.K2_GetRandomLocationInNavigableRadius` (`self.K2_GetActorLocation`) 200.0 null null))
        (`BlackboardComponent.SetValueAsEnum` _blackboard "EActionEnum" (`self.Action`))))))

(event `Attack`)

(event `self.BP_HealthComponent.DamageTaken`)

(event `self.BP_HealthComponent.OnDeath`
  (bind _mesh (`self.Mesh`))
  ;[1 1 1] Death
  (`/Engine/EditorBlueprintResources/StandardMacros.DoOnce` false
    (:`Completed`
      (`PrimitiveComponent.SetCollisionProfileName` (`self.Mesh`) "Ragdoll" true)
      (`SkeletalMeshComponent.SetAllBodiesSimulatePhysics` _mesh true)
      (`PrimitiveComponent.WakeAllRigidBodies` _mesh)
      (`PrimitiveComponent.SetCollisionEnabled` (`self.CapsuleComponent`) "NoCollision"))))

(fn `UserConstructionScript`
  (if (not (`self.bPlayerCharacter`))
    (`SceneComponent.SetVisibility` (`self.NS_Targeting_Player_Select`) true false)))