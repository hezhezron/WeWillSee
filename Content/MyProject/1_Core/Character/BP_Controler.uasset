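; RTS-style player controller that drives the camera pawn and manages unit selection and move orders.
; Input axes and actions pan, yaw, pitch and zoom the camera and its spring arm within clamped limits.
; Left mouse starts and stops HUD selection, clearing selected units when the cursor trace misses.
; CharacterAction spawns a short-lived cursor decal and writes the hit point to each selected unit's Blackboard as TravelLocation.
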(event `self.ReceiveBeginPlay`
  ;[1 1 1] camera movement
  ;;[1 1 1] event begin play/ cast to BPcamera
  (bind _asbp_camera_pawn (cast `/Game/MyProject/2_Character/1_Camera/BP_CameraPawn` (`GameplayStatics.GetPlayerPawn` 0)))
  (set `self.As BP Camera Pawn` _asbp_camera_pawn))

(event `Key|LeftMouseButton`
  (params (Key :type "Key Structure"))
  (bind _returnvalue (`self.GetHUD`))
  ;[1 1 1] character movement
  (:`Pressed`
    (message `/Game/MyProject/1_Core/HUD/BPI_SelectionUnit.StartSelection` _returnvalue)
    (if (not (`.ReturnValue` (`self.GetHitResultUnderCursorByChannel` "TraceTypeQuery3" false)))
      (`self.ClearUnitSelection`)))
  (:`Released`
    (message `/Game/MyProject/1_Core/HUD/BPI_SelectionUnit.StopSelection` _returnvalue)))

(event `InputAxis|rotationCamera`
  (params (AxisValue :type "Float (single-precision)"))
  ;[1 1 1] camera movement
  ;;[1 1 1] Camera rotation
  (`self.K2_SetActorRotation` (`self.As BP Camera Pawn`) (`KismetMathLibrary.MakeRotator` (.roll (`self.K2_GetActorRotation` (`self.As BP Camera Pawn`))) (.pitch (`self.K2_GetActorRotation` (`self.As BP Camera Pawn`))) (+ (.yaw (`self.K2_GetActorRotation` (`self.As BP Camera Pawn`))) (* AxisValue (`self.RotationMultiplicator`)))) false))

(event `InputAxis|MoveForward`
  (params (AxisValue :type "Float (single-precision)"))
  (bind _as_bp_camera_pawn (`self.As BP Camera Pawn`))
  ;[1 1 1] camera movement
  ;;[1 1 1] camera movement
  (`/Engine/EditorBlueprintResources/StandardMacros.IsValid` _as_bp_camera_pawn
    (:`Is Valid`
      (`Pawn.AddMovementInput` _as_bp_camera_pawn (`self.GetActorForwardVector` _as_bp_camera_pawn) (* AxisValue (`self.CameraMovementSpeed`)) false))))

(event `InputAction|CharacterAction`
  (params (Key :type "Key Structure"))
  (bind (_hitresult _returnvalue) (`self.GetHitResultUnderCursorByChannel` "TraceTypeQuery1" false))
  ;[1 1 1] character movement
  (:`Pressed`
    (set `self.Hit Result Location` (`.Location` (`GameplayStatics.BreakHitResult` _hitresult)))
    (if _returnvalue
      (`|ExecutionSequence`
        (:`then_0`
          (if (!= (`KismetArrayLibrary.Array_Length` (`self.SelectedUnit`)) 0)
            (if (`KismetSystemLibrary.IsValid` (`self.ActionDecal`))
              (`ActorComponent.K2_DestroyComponent` (`self.ActionDecal`)))
            (bind _returnvalue_2 (`GameplayStatics.SpawnDecalAtLocation` "/Game/MyProject/5_Effects/Blueprints/M_Cursor_Decal.M_Cursor_Decal" (60.0 60.0 60.0) (`self.Hit Result Location`) (struct :`Pitch` -90.0) 0.5))
            (set `self.ActionDecal` _returnvalue_2)))
        (:`then_1`
          (for _array_element (`self.SelectedUnit`)
            (`BlackboardComponent.SetValueAsVector` (`AIBlueprintHelperLibrary.GetBlackboard` _array_element) "TravelLocation" (`self.Hit Result Location`))))))))

(event `InputAxis|MoveRight`
  (params (AxisValue :type "Float (single-precision)"))
  (bind _as_bp_camera_pawn (`self.As BP Camera Pawn`))
  ;[1 1 1] camera movement
  ;;[1 1 1] camera movement
  (`Pawn.AddMovementInput` _as_bp_camera_pawn (`self.GetActorRightVector` _as_bp_camera_pawn) (* AxisValue (`self.CameraMovementSpeed`)) false))

(event `InputAxis|LookUp`
  (params (AxisValue :type "Float (single-precision)"))
  ;[1 1 1] camera movement
  ;;[1 1 1] campera pitch
  (`SceneComponent.K2_SetRelativeRotation` (`/Game/MyProject/2_Character/1_Camera/BP_CameraPawn.SpringArm` (`self.As BP Camera Pawn`)) (`KismetMathLibrary.MakeRotator` (.roll (`SceneComponent.RelativeRotation` (`/Game/MyProject/2_Character/1_Camera/BP_CameraPawn.SpringArm` (`self.As BP Camera Pawn`)))) (`KismetMathLibrary.ClampAngle` (+ (* AxisValue (`self.CameraPitchSpeed`)) (.pitch (`SceneComponent.RelativeRotation` (`/Game/MyProject/2_Character/1_Camera/BP_CameraPawn.SpringArm` (`self.As BP Camera Pawn`))))) (`self.MinAngleDegrees`) (`self.Max Angle Degrees`)) (.yaw (`SceneComponent.RelativeRotation` (`/Game/MyProject/2_Character/1_Camera/BP_CameraPawn.SpringArm` (`self.As BP Camera Pawn`))))) false false))

(event `InputAction|ZoomIn`
  (params (Key :type "Key Structure"))
  ;[1 1 1] camera movement
  ;;[1 0.8404 0.02372] zoom (to correct)
  (:`Pressed`
    (set `SpringArmComponent.TargetArmLength` (`KismetMathLibrary.FClamp` (- (`SpringArmComponent.TargetArmLength` (`/Game/MyProject/2_Character/1_Camera/BP_CameraPawn.SpringArm` (`self.As BP Camera Pawn`))) (`self.CameraZoomSpeed`)) (`self.ZoomMin`) (`self.ZomMax`)) (`/Game/MyProject/2_Character/1_Camera/BP_CameraPawn.SpringArm` (`self.As BP Camera Pawn`)))))

(event `InputAction|ZoomOut`
  (params (Key :type "Key Structure"))
  ;[1 1 1] camera movement
  ;;[1 0.8404 0.02372] zoom (to correct)
  (:`Pressed`
    (set `SpringArmComponent.TargetArmLength` (`KismetMathLibrary.FClamp` (+ (`SpringArmComponent.TargetArmLength` (`/Game/MyProject/2_Character/1_Camera/BP_CameraPawn.SpringArm` (`self.As BP Camera Pawn`))) (`self.CameraZoomSpeed`)) (`self.ZoomMin`) (`self.ZomMax`)) (`/Game/MyProject/2_Character/1_Camera/BP_CameraPawn.SpringArm` (`self.As BP Camera Pawn`)))))

(fn `AddUnitSelection`
  (params (Character :type "/Game/MyProject/1_Core/Character/BP_Character Object Reference"))
  (`KismetArrayLibrary.Array_AddUnique` (`self.SelectedUnit`) Character)
  (`/Game/MyProject/1_Core/Character/BP_Character.UnitSelected` Character true))

(fn `ClearUnitSelection`
  (for _array_element (`self.SelectedUnit`)
    (bind _asbp_character (cast `/Game/MyProject/1_Core/Character/BP_Character` _array_element))
    (`/Game/MyProject/1_Core/Character/BP_Character.UnitSelected` _asbp_character false))
  (`KismetArrayLibrary.Array_Clear` (`self.SelectedUnit`)))

(fn `DeleteUnitSelection`
  (params (Character :type "/Game/MyProject/1_Core/Character/BP_Character Object Reference"))
  (`KismetArrayLibrary.Array_RemoveItem` (`self.SelectedUnit`) Character)
  (`/Game/MyProject/1_Core/Character/BP_Character.UnitSelected` Character false))

(fn `UserConstructionScript`)