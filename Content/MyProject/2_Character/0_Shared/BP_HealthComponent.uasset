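; BP_HealthComponent is a shared component that tracks the owning actor's health and announces damage and death.
; On BeginPlay it fills current health to max and binds to the owner's OnTakeAnyDamage event.
; Positive damage fires DamageTaken before being subtracted from current health, then OnDeath fires if IsDead finds health at or below zero.
; Health is not clamped, and further hits after death can fire OnDeath again.
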(event `self.ReceiveBeginPlay`
  (set `self.CurrentHealth` (`self.MaxHealth`))
  (add `Actor.OnTakeAnyDamage` (`self.GetOwner`) (delegate `OnTakeAnyDamage_Event_0`)))

(event `OnTakeAnyDamage_Event_0`
  (params (DamagedActor :type "Actor Object Reference") (Damage :type "Float (double-precision)") (DamageType :type "DamageType Object Reference") (InstigatedBy :type "Controller Object Reference") (DamageCauser :type "Actor Object Reference"))
  (if (> Damage 0.0)
    (`self.DamageTaken`)
    (set `self.CurrentHealth` (- (`self.CurrentHealth`) Damage))
    (if (`self.IsDead`)
      (`self.OnDeath`))))

(fn `IsDead`
  (returns (Dead :type Boolean))
  (return (<= (`self.CurrentHealth`) 0.0)))